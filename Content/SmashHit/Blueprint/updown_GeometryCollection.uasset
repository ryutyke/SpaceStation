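; A SmashHit obstacle that moves up and down until it is hit, built around a Geometry Collection and a Box collider.
; Each Tick, while Hit is false, it flips GoDown at fixed upper and lower world-Z limits and applies a fixed local-Z offset without sweep, so speed depends on frame rate.
; A Box hit enables physics simulation on the Geometry Collection, sets Hit to stop the movement, and destroys the Box.
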(event OnComponentHit(Box)
  (params (HitComponent :type Primitive%20Component%20Object%20Reference) (OtherActor :type Actor%20Object%20Reference) (OtherComp :type Primitive%20Component%20Object%20Reference) (NormalImpulse :type Vector :default "0, 0, 0") (Hit :type Hit%20Result%20Structure%20%28by%20ref%29))
  ;[1 1 1] 맞으면 멈춰있어야한다.
  (Physics|SetSimulatePhysics (Variables|Default|GetGeometryCollection) true)
  (bind _output_get (Variables|Default|Sethit? true))
  (Components|DestroyComponent (Variables|Default|GetBox)))

(event EventBeginPlay)

(event Collision|EventActorBeginOverlap
  (params (OtherActor :type Actor%20Object%20Reference)))

(event EventTick
  (params (DeltaSeconds :type Float%20%28single-precision%29))
  (bind _returnvalue (Transformation|GetActorLocation))
  ;[1 1 1] 상하 이동(Go Down의 초기값을 False로 한다면 시작시 위부터 감)
  (if (not (stale OnComponentHit(Box) _output_get))
    (Utilities|FlowControl|Sequence
      (:then_0
        (if (>= (.z _returnvalue) 2.1e+02)
          (bind _output_get (Variables|Default|SetGo%20Down true))
          (elif (<= (.z _returnvalue) -1.1e+02)
            (Variables|Default|SetGo%20Down false))))
      (:then_1
        (if _output_get
          (Transformation|AddActorLocalOffset "0.000000,0.000000,-3.000000" false false)
          (else
            (Transformation|AddActorLocalOffset "0.000000,0.000000,3.000000" false false)))))))

(fn ConstructionScript)